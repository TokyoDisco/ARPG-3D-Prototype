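; Damage dummy enemy that loses health when hit and can draw the player into battle.
; An EnemyStats component holds health, randomizes the name at BeginPlay and grants experience to TargetPlayer on death.
; DetectionZone overlaps add or remove it from the player's EnemyArray, set or clear TargetPlayer, and call BattleEntering both ways.
; Tick polls health, spawning an explosion and destroying the actor at zero or below.
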(event OnComponentBeginOverlap(DetectionZone)
  (params (OverlappedComponent :type Primitive%20Component%20Object%20Reference) (OtherActor :type Actor%20Object%20Reference) (OtherComp :type Primitive%20Component%20Object%20Reference) (OtherBodyIndex :type Integer) (bFromSweep :type Boolean) (SweepResult :type Hit%20Result%20Structure%20%28by%20ref%29))
  ;[1 1 1] Call for Player oject to enter battle
  (CallFunction|BattleZoneEntering OtherActor))

(event OnComponentEndOverlap(DetectionZone)
  (params (OverlappedComponent :type Primitive%20Component%20Object%20Reference) (OtherActor :type Actor%20Object%20Reference) (OtherComp :type Primitive%20Component%20Object%20Reference) (OtherBodyIndex :type Integer))
  ;[1 1 1] Call for Player oject to enter battle
  (CallFunction|BattleZoneLeaving OtherActor))

(event Collision|EventActorBeginOverlap
  (params (OtherActor :type Actor%20Object%20Reference)))

(event Game|Damage|EventAnyDamage
  (params (Damage :type Float%20%28single-precision%29) (DamageType :type Damage%20Type%20Object%20Reference) (InstigatedBy :type Controller%20Object%20Reference) (DamageCauser :type Actor%20Object%20Reference))
  (bind _enemystats (Variables|Default|GetEnemyStats))
  ;[1 1 1] Taking Damage Event
  (Variables|/Game/Blueprints/EnemyStats.EnemyStats_C|SetHealthPoints _enemystats (- (Variables|/Game/Blueprints/EnemyStats.EnemyStats_C|GetHealthPoints _enemystats) Damage)))

(event EventTick
  (params (DeltaSeconds :type Float%20%28single-precision%29))
  ;[1 1 1] Death Detection and spawning death effect
  (Math|Float|CompareFloat (Variables|/Game/Blueprints/EnemyStats.EnemyStats_C|GetHealthPoints (Variables|Default|GetEnemyStats)) 0.0
    (:==
      _)
    (:<
      _))
  (Default|ExperienceReward (Variables|Default|GetEnemyStats) (Variables|Default|GetTargetPlayer))
  (Effects|SpawnEmitteratLocation "/Game/StarterContent/Particles/P_Explosion.P_Explosion" (Transformation|GetActorLocation) "0,0.000000, 0")
  (Actor|DestroyActor))

(event EventBeginPlay
  ;[1 1 1] Name Randomizer
  (Default|NameRandomizer (Variables|Default|GetEnemyStats)))

(fn ConstructionScript)

(fn BattleZoneEntering
  (params (Player :type Actor%20Object%20Reference))
  (bind _returnvalue (Game|Player|GetPlayerPawn 0))
  (if (Actor|ActorHasTag Player "Player")
    (bind _asthird_person_character (Utilities|Casting|CastToThirdPersonCharacter _returnvalue))
    (Utilities|Array|Add (Variables|/Game/ThirdPersonBP/Blueprints/ThirdPersonCharacter.ThirdPersonCharacter_C|GetEnemyArray _asthird_person_character) self)
    (Default|BattleEntering _asthird_person_character)
    (Variables|Default|SetTargetPlayer _returnvalue)))

(fn BattleZoneLeaving
  (params (Player :type Actor%20Object%20Reference))
  (if (Actor|ActorHasTag Player "Player")
    (bind _asthird_person_character (Utilities|Casting|CastToThirdPersonCharacter (Game|Player|GetPlayerPawn 0)))
    (Utilities|Array|RemoveItem (Variables|/Game/ThirdPersonBP/Blueprints/ThirdPersonCharacter.ThirdPersonCharacter_C|GetEnemyArray _asthird_person_character) self)
    (Default|BattleEntering _asthird_person_character)
    (Variables|Default|SetTargetPlayer 0)))