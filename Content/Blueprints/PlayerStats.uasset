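; Player stats Blueprint that manages health, mana, potions, experience, levelling and skill casting.
; Experience gain triggers a level check, which adds MoonLightStream to the skill list at level 2.
; UseSkill reads class defaults for cost and cooldown, then spawns the skill actor at the player, aimed along the camera boom.
; Tick quits the game at zero health and clears only slot 1's cooldown; the DEV fireball logic is disconnected.
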(event EventBeginPlay)

(event EventTick
  (params (DeltaSeconds :type Float%20%28single-precision%29))
  ;[1 0.14 0.14] Health Check
  (Math|Float|CompareFloat (Variables|Default|GetHealthPoints) 0.0 :!label _label
    (:>
      (if (Variables|Default|GetSkill1onCD)
        (Utilities|FlowControl|Delay (Variables|Default|GetSkill1CD))
        (Variables|Default|SetSkill1onCD false)
        (goto _label)))
    (:==
      (Game|QuitGame 0 "Quit" :!label _label_2))
    (:<
      (goto _label_2))))

(fn ManaRechargePotion
  (params (ManaAmount :type Float%20%28single-precision%29))
  (bind _maxmana (Variables|Default|GetMaxMana))
  (bind _output_get (Variables|Default|SetManaPoints (+ ManaAmount (Variables|Default|GetManaPoints))))
  (Math|Float|CompareFloat _output_get _maxmana
    (:>
      (Variables|Default|SetManaPoints _maxmana))))

(fn HealRechargePotion
  (params (HealAmount :type Float%20%28single-precision%29))
  (bind _maxhp (Variables|Default|GetMaxHp))
  (bind _output_get (Variables|Default|SetHealthPoints (+ (Variables|Default|GetHealthPoints) HealAmount)))
  (Math|Float|CompareFloat _output_get _maxhp
    (:>
      _)
    (:==
      _))
  (Variables|Default|SetHealthPoints _maxhp))

(fn TakeDamageNormal
  (params (DamageAmount :type Float%20%28single-precision%29))
  (Variables|Default|SetHealthPoints (- (Variables|Default|GetHealthPoints) DamageAmount)))

(fn DEVFireballSkillID0)

(fn LevelUpCheck
  (Math|Integer|CompareInt (Variables|Default|GetExperiencesPoints) (Variables|Default|GetReqExp)
    (:>
      _)
    (:==
      _))
  (Variables|Default|SetLevel (+ (Variables|Default|GetLevel) 1))
  (Variables|Default|SetExperiencesPoints (- (Variables|Default|GetExperiencesPoints) (Variables|Default|GetReqExp)))
  (switch int (Variables|Default|GetLevel)
    (:2
      (bind _output_get (Variables|Default|SetSkillList (Variables|Default|GetSkillList)))
      (Utilities|Array|Add _output_get "/Game/Blueprints/SkillsClass/MoonLightStream.MoonLightStream_C"))))

(fn ExperienceGain
  (params (ExpAmount :type Integer))
  (Variables|Default|SetExperiencesPoints (+ (Variables|Default|GetExperiencesPoints) ExpAmount))
  (CallFunction|LevelUpCheck))

(fn UseSkill
  (params (SkillActor :type Skill%20Stats%20Class%20Reference) (Slot :type Integer))
  (bind _returnvalue (Game|Player|GetPlayerPawn 0))
  (bind (_damage _cost _type _name _elemental _descirption _areaeffectflag _upgrade _skill_id _cooldown _skillactorclass) (Utilities|GetClassDefaults SkillActor))
  (bind _returnvalue_2 (Math|Conversions|ToFloat(Integer) _cooldown))
  (Math|Float|CompareFloat (Variables|Default|GetManaPoints) _cost
    (:>
      _)
    (:==
      _))
  (Variables|Default|SetManaPoints (- (Variables|Default|GetManaPoints) _cost))
  (switch int Slot
    (:Default
      (Variables|Default|SetSkill1CD _returnvalue_2 :!label _label)
      (Variables|Default|SetSkill1onCD true))
    (:0
      (goto _label))
    (:1
      (goto _label))
    (:2
      (Variables|Default|SetSkill2CD _returnvalue_2)
      (Variables|Default|SetSkill2onCD true))
    (:3
      (Variables|Default|SetSkill3CD _returnvalue_2)
      (Variables|Default|SetSkill3onCD true))
    (:4
      (Variables|Default|SetSkill4CD _returnvalue_2)
      (Variables|Default|SetSkill4onCD true)))
  (bind _asthird_person_character (Utilities|Casting|CastToThirdPersonCharacter _returnvalue))
  (Game|SpawnActorfromClass _skillactorclass (Math|Transform|MakeTransform (Transformation|GetActorLocation _returnvalue) (Transformation|GetWorldRotation (Variables|/Game/ThirdPersonBP/Blueprints/ThirdPersonCharacter.ThirdPersonCharacter_C|GetCameraBoom _asthird_person_character))) "Undefined" 0 0)
  (bind _output_get (Variables|/Game/ThirdPersonBP/Blueprints/ThirdPersonCharacter.ThirdPersonCharacter_C|SetSkillName _asthird_person_character _name))
  (Variables|/Game/ThirdPersonBP/Blueprints/ThirdPersonCharacter.ThirdPersonCharacter_C|SetLastUsedSkill _asthird_person_character _output_get))