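; Fireball test skill projectile that damages what it hits and homes in on the player's active target.
; Each Tick, while the ThirdPersonCharacter's EnemyArray is non-empty, it sets the homing target to the ActiveTarget's StaticMeshComponent.
; A sphere hit on a non-Player actor applies damage credited to the player pawn, plays audio and particles, then destroys the projectile after a brief delay.
; It also self-destructs after a fixed lifetime.
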(event OnComponentHit(Sphere)
  (params (HitComponent :type Primitive%20Component%20Object%20Reference) (OtherActor :type Actor%20Object%20Reference) (OtherComp :type Primitive%20Component%20Object%20Reference) (NormalImpulse :type Vector :default "0, 0, 0") (Hit :type Hit%20Result%20Structure%20%28by%20ref%29))
  (if (not (Actor|ActorHasTag OtherActor "Player"))
    (Game|Damage|ApplyDamage OtherActor (Variables|Default|GetBaseDmg) 0 (Game|Player|GetPlayerPawn 0))
    (Audio|Components|Audio|Play (Variables|Default|GetAudio1) 0.0)
    (Components|Activation|Activate (Variables|Default|GetParticleSystem1) false)
    (Utilities|FlowControl|Delay 0.3)
    (Actor|DestroyActor)))

(event Collision|EventActorBeginOverlap
  (params (OtherActor :type Actor%20Object%20Reference)))

(event EventBeginPlay
  (Utilities|FlowControl|Delay 3.0)
  (Actor|DestroyActor))

(event EventTick
  (params (DeltaSeconds :type Float%20%28single-precision%29))
  (bind _asthird_person_character (Utilities|Casting|CastToThirdPersonCharacter (Game|Player|GetPlayerPawn 0)))
  (Math|Integer|CompareInt (Utilities|Array|Length (Variables|/Game/ThirdPersonBP/Blueprints/ThirdPersonCharacter.ThirdPersonCharacter_C|GetEnemyArray _asthird_person_character)) 0
    (:>
      (Variables|/Script/Engine.ProjectileMovementComponent|SetHomingTargetComponent (Variables|Default|GetProjectileMovement) (Actor|GetComponentbyClass (Variables|/Game/ThirdPersonBP/Blueprints/ThirdPersonCharacter.ThirdPersonCharacter_C|GetActive%20Target _asthird_person_character) "/Script/Engine.StaticMeshComponent")))))

(fn ConstructionScript)