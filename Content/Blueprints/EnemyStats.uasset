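; EnemyStats is an actor component that holds an enemy's health, name and experience value.
; DeathDetection destroys the owning actor when health is below zero, and NameRandomizer picks a random name from an array.
; ExperienceReward passes the experience value to the given player's PlayerStats component.
; The event graph has no active logic, and none of these functions is called within the file.
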(event EventBeginPlay)

(event EventTick
  (params (DeltaSeconds :type Float%20%28single-precision%29)))

(fn DeathDetection
  (Math|Float|CompareFloat (Variables|Default|GetHealthPoints) 0.0
    (:<
      (Actor|DestroyActor (Components|GetOwner)))))

(fn NameRandomizer
  (bind _namesarray (LocalVariables|GetNamesArray))
  (Variables|Default|SetName (Utilities|Array|Get(acopy) _namesarray (Math|Random|RandomIntegerinRange 0 (Utilities|Array|LastIndex _namesarray)))))

(fn ExperienceReward
  (params (PlayerToReward :type Actor%20Object%20Reference))
  (Default|ExperienceGain (Actor|GetComponentbyClass PlayerToReward "/Game/Blueprints/PlayerStats.PlayerStats_C") (Variables|Default|GetExperience)))