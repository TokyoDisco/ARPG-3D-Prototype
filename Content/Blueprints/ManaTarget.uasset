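; ManaTarget is a development target for projectile testing that alters the player's stats when hit by a skill.
; When an actor tagged Skill overlaps its Box, it gets player 0's ThirdPersonCharacter and switches on the parent actor's object name.
; That name selects whether PlayerStats applies a mana recharge, a heal or normal damage to the player.
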(event OnComponentBeginOverlap(Box)
  (params (OverlappedComponent :type Primitive%20Component%20Object%20Reference) (OtherActor :type Actor%20Object%20Reference) (OtherComp :type Primitive%20Component%20Object%20Reference) (OtherBodyIndex :type Integer) (bFromSweep :type Boolean) (SweepResult :type Hit%20Result%20Structure%20%28by%20ref%29))
  ;[1 1 1] DEV Projectile Testing Area
  (if (Actor|ActorHasTag OtherActor "Skill")
    (bind _asthird_person_character (Utilities|Casting|CastToThirdPersonCharacter (Game|Player|GetPlayerPawn 0)))
    (switch string (Utilities|GetObjectName (Actor|GetParentActor))
      (:ManaRecharge
        (Default|ManaRechargePotion (Variables|/Game/ThirdPersonBP/Blueprints/ThirdPersonCharacter.ThirdPersonCharacter_C|GetPlayerStats _asthird_person_character) 5e+01))
      (:HealRecharge
        (Default|HealRechargePotion (Variables|/Game/ThirdPersonBP/Blueprints/ThirdPersonCharacter.ThirdPersonCharacter_C|GetPlayerStats _asthird_person_character) 1e+01))
      (:DamageDummy
        (Default|TakeDamageNormal (Variables|/Game/ThirdPersonBP/Blueprints/ThirdPersonCharacter.ThirdPersonCharacter_C|GetPlayerStats _asthird_person_character) 15.0)))))

(event EventBeginPlay)

(event Collision|EventActorBeginOverlap
  (params (OtherActor :type Actor%20Object%20Reference)))

(event EventTick
  (params (DeltaSeconds :type Float%20%28single-precision%29)))

(fn ConstructionScript)